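; BP_AI_ENEMYBOSS is the AI controller for the boss enemy, BP_AI_BOSS.
; On BeginPlay it caches the controlled boss and runs the BT_Boss behavior tree unless the boss's combat component reports it dead.
; When PawnSensing sees a pawn, it writes that pawn and a seeing-target flag to the Blackboard, and nothing here clears them.
; A disconnected node for playing 2D organ music never runs.
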(event `self.ReceiveBeginPlay`
  (bind _asbp_ai_boss (cast `/Game/AI/BP_AI_BOSS` (`self.K2_GetPawn`)))
  (bind _output_get (set `self.As BP AI BOSS` _asbp_ai_boss))
  (if (not (`/Game/BluePrints/BPC_BOSSCombat.isDead?` (`/Game/AI/BP_AI_BOSS.BPC_BOSSCombat` _output_get)))
    (`self.RunBehaviorTree` "/Game/AI/BT_Boss.BT_Boss")))

(event `self.PawnSensing.OnSeePawn`
  (params (Pawn :type "Pawn Object Reference"))
  (`BlackboardComponent.SetValueAsBool` (`AIBlueprintHelperLibrary.GetBlackboard` null) "seeingTarget?" true)
  (`BlackboardComponent.SetValueAsObject` (`AIBlueprintHelperLibrary.GetBlackboard` null) "target" Pawn))

(fn `UserConstructionScript`)