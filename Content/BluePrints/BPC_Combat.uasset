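; Player combat component for BP_ThirdPersonREV that handles free aim, target lock and stamina-based dodge rolls.
; Free aim offsets the camera and switches to controller-driven rotation while held.
; Lock toggles on a camera-forward sphere-traced pawn, attaches a marker actor and steers control rotation toward it each tick.
; Dodge requires speed and stamina, picks a montage by direction key when controller-rotated, and pauses stamina regen until it ends.
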(event `self.ReceiveBeginPlay`
  ; Get Player Class
  (bind _asbp_third_person_rev (cast `/Game/Characters/REV/BP_ThirdPersonREV` (`self.GetOwner`)))
  (set `self.BP Third Person REV` _asbp_third_person_rev))

(event `EnhancedInput|/Game/Input/Actions/IA_FreeAim`
  (params (ActionValue :type Boolean) (ElapsedSeconds :type "Float (double-precision)") (TriggeredSeconds :type "Float (double-precision)") (InputAction :type "InputAction Object Reference" :default "/Game/Input/Actions/IA_FreeAim.IA_FreeAim"))
  (bind _cameraboom (`/Game/Characters/REV/BP_ThirdPersonREV.CameraBoom` (`self.BP Third Person REV`)))
  (bind _followcamera (`/Game/Characters/REV/BP_ThirdPersonREV.FollowCamera` (`self.BP Third Person REV`)))
  (bind _charactermovement (`Character.CharacterMovement` (`self.BP Third Person REV`)))
  ;[0 0 0] FreeAim
  (:`Triggered`
    (if true
      (set `self.isAiming?` true)
      (set `CharacterMovementComponent.bOrientRotationToMovement` false _charactermovement)
      (set `CharacterMovementComponent.bUseControllerDesiredRotation` true _charactermovement)
      (set `SpringArmComponent.SocketOffset` (210.0 82.0 70.0) _cameraboom)
      (`SceneComponent.K2_SetRelativeRotation` _followcamera (struct :`Pitch` -16.0) false false)))
  (:`Completed`
    (set `self.isAiming?` false)
    (set `CharacterMovementComponent.bOrientRotationToMovement` true _charactermovement)
    (set `CharacterMovementComponent.bUseControllerDesiredRotation` false _charactermovement)
    (set `SpringArmComponent.SocketOffset` (0.0 0.0 0.0) _cameraboom)
    (`SceneComponent.K2_SetRelativeRotation` :`self` _followcamera)))

(event `EnhancedInput|/Game/Input/Actions/IA_Lock`
  (params (ActionValue :type Boolean) (ElapsedSeconds :type "Float (double-precision)") (TriggeredSeconds :type "Float (double-precision)") (InputAction :type "InputAction Object Reference" :default "/Game/Input/Actions/IA_Lock.IA_Lock"))
  (bind _returnvalue (`Actor.GetTransform` (`self.Target Lock Actor`)))
  (bind _transformcomponent (`PlayerCameraManager.TransformComponent` (`GameplayStatics.GetPlayerCameraManager` 0)))
  (bind _charactermovement (`Character.CharacterMovement` (`self.BP Third Person REV`)))
  (bind _charactermovement_2 (`Character.CharacterMovement` (`self.BP Third Person REV`)))
  (bind (_returnvalue_x _returnvalue_y _returnvalue_z) (`KismetMathLibrary.BreakVector` (`SceneComponent.K2_GetComponentLocation` _transformcomponent)))
  (bind _returnvalue_2 (`KismetMathLibrary.MakeVector` _returnvalue_x _returnvalue_y (+ _returnvalue_z 40.0)))
  ;[0 0 0] Target Lock
  (:`Started`
    (`self.Target Lock Actor`
      (:`then`
        (set `self.Target Lock Actor` null)
        (set `CharacterMovementComponent.bOrientRotationToMovement` true _charactermovement)
        (set `CharacterMovementComponent.bUseControllerDesiredRotation` false _charactermovement)
        (`Actor.K2_DestroyActor` (`self.Target Lock Widget`)))
      (:`else`
        (bind (_outhit _returnvalue_3) (`KismetSystemLibrary.SphereTraceSingleForObjects` :`Start` _returnvalue_2 :`End` (+ _returnvalue_2 (* (`KismetMathLibrary.GetForwardVector` (`SceneComponent.K2_GetComponentRotation` _transformcomponent)) 2000.0)) :`Radius` 150.0 :`ObjectTypes` (`|MakeArray` "ObjectTypeQuery3" :!type "EObjectTypeQuery Enum") :`DrawDebugType` "ForDuration" :`DrawTime` 2.0))
        (if _returnvalue_3
          (set `self.Target Lock Actor` (`.HitActor` (`GameplayStatics.BreakHitResult` _outhit)))
          (set `CharacterMovementComponent.bOrientRotationToMovement` false _charactermovement_2)
          (set `CharacterMovementComponent.bUseControllerDesiredRotation` true _charactermovement_2)
          (bind _returnvalue_4 (`|SpawnActorFromClass` "/Game/BluePrints/BP_TargetLockWidget.BP_TargetLockWidget_C" (`KismetMathLibrary.MakeTransform` (`KismetMathLibrary.MakeVector` (.x (.location _returnvalue)) (.y (.location _returnvalue)) (+ (.z (.location _returnvalue)) 40.0)) (.rotation _returnvalue)) "AlwaysSpawn" "MultiplyWithRoot" null null))
          (bind _output_get (set `self.Target Lock Widget` _returnvalue_4))
          (`Actor.K2_AttachToActor` _output_get (`self.Target Lock Actor`) "None" "SnapToTarget" "KeepRelative" "KeepRelative" true))))))

(event `self.ReceiveTick`
  (params (DeltaSeconds :type "Float (single-precision)"))
  (bind (_returnvalue_roll _returnvalue_pitch _returnvalue_yaw) (`KismetMathLibrary.BreakRotator` (`KismetMathLibrary.FindLookAtRotation` (`Actor.K2_GetActorLocation` (`self.BP Third Person REV`)) (`Actor.K2_GetActorLocation` (`self.Target Lock Actor`)))))
  ;[0 0 0] Target Lock Update
  (`self.Target Lock Actor`
    (:`then`
      (`Controller.SetControlRotation` (`Pawn.GetController` (`self.BP Third Person REV`)) (`KismetMathLibrary.MakeRotator` _returnvalue_roll (+ _returnvalue_pitch -20.0) _returnvalue_yaw)))
    (:`else`)))

(event `EnhancedInput|/Game/Input/Actions/IA_Dodge`
  (params (ActionValue :type Boolean) (ElapsedSeconds :type "Float (double-precision)") (TriggeredSeconds :type "Float (double-precision)") (InputAction :type "InputAction Object Reference" :default "/Game/Input/Actions/IA_Dodge.IA_Dodge"))
  (bind _velocity (`MovementComponent.Velocity` (`Character.CharacterMovement` (`self.BP Third Person REV`))))
  ;[0 0 0 0.5] Dodging
  (:`Started`
    (if (and (not (`self.isDodging`)) (>= (`KismetMathLibrary.VSize` _velocity) 400.0) (>= (`KismetAnimationLibrary.CalculateDirection` _velocity (`Actor.K2_GetActorRotation` (`self.BP Third Person REV`))) 0.0) (> (`/Game/BluePrints/BPC_Stats.Stamina` (`/Game/Characters/REV/BP_ThirdPersonREV.BPC_Stats` (`self.BP Third Person REV`))) 25.0))
      (set `self.isDodging` true)
      (`|ExecutionSequence`
        (:`then_0`
          (if (`CharacterMovementComponent.bUseControllerDesiredRotation` (`Character.CharacterMovement` (`self.BP Third Person REV`)))
            (switch `string` (`KismetTextLibrary.Conv_TextToString` (`KismetInputLibrary.Key_GetDisplayName` (`/Game/Characters/REV/BP_ThirdPersonREV.Direction Key` (`self.BP Third Person REV`))))
              (:`W`
                (set `self.movementDirection` "NewEnumerator0"))
              (:`A`
                (set `self.movementDirection` "NewEnumerator1"))
              (:`S`
                (set `self.movementDirection` "NewEnumerator2"))
              (:`D`
                (set `self.movementDirection` "NewEnumerator3")))
            (else
              (set `self.movementDirection` "NewEnumerator0"))))
        (:`then_1`
          (`|PlayMontage` (`Character.Mesh` (`self.BP Third Person REV`)) (select `/Game/BluePrints/E_MovementDirection` (`self.movementDirection`) :`NewEnumerator0` "/Game/Characters/REV/Animations/Roll_Montage.Roll_Montage" :`NewEnumerator1` "/Game/Characters/REV/Animations/Roll_Montage.Roll_Montage" :`NewEnumerator3` "/Game/Characters/REV/Animations/Roll_Montage.Roll_Montage" :!type "AnimMontage Object Reference")
            (:`then`
              (set `/Game/BluePrints/BPC_Stats.regenStamina?` false (`/Game/Characters/REV/BP_ThirdPersonREV.BPC_Stats` (`self.BP Third Person REV`)))
              (`/Game/BluePrints/BPC_Stats.Increase Value` (`/Game/Characters/REV/BP_ThirdPersonREV.BPC_Stats` (`self.BP Third Person REV`)) "NewEnumerator1" -25.0))
            (:`OnCompleted`
              (set `self.isDodging` false :!label _label)
              (set `/Game/BluePrints/BPC_Stats.regenStamina?` true (`/Game/Characters/REV/BP_ThirdPersonREV.BPC_Stats` (`self.BP Third Person REV`))))
            (:`OnInterrupted`
              (goto _label))))))))